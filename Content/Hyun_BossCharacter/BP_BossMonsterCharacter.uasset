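; Boss monster character that plays named attack and reaction montages, fires projectiles, slowly regenerates health and shows the HUD win state on death.
; BeginPlay registers montages in a name map, suffixing list entries with their index; OnPlayMontage looks them up and relays completion, blend-out, interrupt and notify callbacks.
; Core breaks set per-thread scalars on a dynamic mesh material.
; Gun-counter handling only prints; hit-trace debugging is unbound.
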(event Custom|OnHitStartEvent_Event_0
  (params (hitResult :type Hit%20Result%20Structure%20%28by%20ref%29) (Causer :type Actor%20Object%20Reference) (Type :type Object%20Class%20Reference))
  (bind (_bblockinghit _binitialoverlap _time _distance _location _impactpoint _normal _impactnormal _physmat _hitactor _hitcomponent _hitbonename _hititem _elementindex _faceindex _tracestart) (Collision|BreakHitResult hitResult))
  (if _bblockinghit
    (Collision|BoxTraceByChannel _impactpoint _impactpoint "5.000000,5.000000,5.000000" "0, 0, 0" "TraceTypeQuery1" false 0 "ForDuration" true "(R=0.000000,G=0.000000,B=0.000000,A=1.000000)")
    (Collision|BoxTraceByChannel _tracestart _tracestart "5.000000,5.000000,5.000000" "0, 0, 0" "TraceTypeQuery1" false 0 "ForDuration" true "(R=0.315391,G=1.000000,B=0.000000,A=1.000000)")))

(event Custom|OnDeadEvent_Event_0
  (bind _asbp_huddefault (Utilities|Casting|CastToBP_HUDDefault (HUD|GetHUD (Game|GetPlayerController 0))))
  (Default|OnWin _asbp_huddefault))

(event Custom|OnPlayAnimMontage
  (params (Montage :type Anim%20Montage%20Object%20Reference) (StartPosition :type Float%20%28single-precision%29))
  (bind _notifyname (Animation|Montage|PlayMontage (Variables|Character|GetMesh) Montage 1.0 StartPosition)
    (:OnCompleted
      (Class|CharacterMaster|OnAnimCompleted))
    (:OnBlendOut
      (Class|CharacterMaster|OnAnimBlendOut))
    (:OnInterrupted
      (Class|CharacterMaster|OnAnimInterrupted))
    (:OnNotifyBegin
      (Class|CharacterMaster|OnAnimNotifyBegin _notifyname))))

(event Custom|OnGunCounterStartEvent_Event_0
  (Development|PrintString "Hello"))

(event EventBeginPlay
  (bind _cables (Variables|Default|GetCables))
  (Utilities|FlowControl|Sequence
    (:then_0
      (CallFunction|AddMontage (Variables|Default|GetAnimMontageNameHit) (Variables|애니메이션|GetHitAnimMontage))
      (CallFunction|AddMontage (Variables|Default|GetAnimMontageNameAttackNormal) (Variables|애니메이션|GetAttackNormalAnimMontage))
      (CallFunction|AddMontage (Variables|Default|GetAnimMontageNameAttack01) (Variables|애니메이션|GetAttack01AnimMontage))
      (CallFunction|AddMontage (Variables|Default|GetAnimMontageNameAttack01Strong) (Variables|애니메이션|GetAttack01StrongAnimMontage))
      (CallFunction|AddMontage (Variables|Default|GetAnimMontageNameAttack01Danger) (Variables|애니메이션|GetAttack01DangerAnimMontage))
      (CallFunction|AddMontage (Variables|Default|GetAnimMontageNameAttack02) (Variables|애니메이션|GetAttack02AnimMontage))
      (CallFunction|AddMontage (Variables|Default|GetAnimMontageNameAttack02Danger) (Variables|애니메이션|GetAttack02DangerAnimMontage))
      (CallFunction|AddMontage (Variables|Default|GetAnimMontageNameAttackShoot) (Variables|애니메이션|GetAttackShootAnimMontage))
      (CallFunction|AddMontage (Variables|Default|GetAnimMontageNameDodge) (Variables|Default|GetDodgeAnimMontage)))
    (:then_1
      (CallFunction|AddMontageList (Variables|Default|GetAnimMontageNameParry) (Variables|애니메이션|GetParryAnimMontages))
      (CallFunction|AddMontageList (Variables|Default|GetAnimMontageNameGroggy) (Variables|애니메이션|GetGroggyAnimMontages))
      (CallFunction|AddMontageList (Variables|Default|GetAnimMontageNameAttackJump) (Variables|애니메이션|GetAttackJumpAnimMontage))
      (CallFunction|AddMontageList (Variables|Default|GetAnimMontageNameAttackFail) (Variables|애니메이션|GetAttackFailAnimMontages))
      (CallFunction|AddMontageList (Variables|Default|GetAnimMontageNameCoreBrake) (Variables|애니메이션|GetCoreBrakeAnimMontages))
      (CallFunction|AddMontageList (Variables|Default|GetAnimMontageNameAttackRush) (Variables|애니메이션|GetAttackRushAnimMontage))
      (bind _asplayer_character (Utilities|Casting|CastToPlayerCharacter (Game|Player|GetPlayerPawn 0)))
      (EventDispatchers|AssignOnGunCounterStartEvent _asplayer_character (delegate Custom|OnGunCounterStartEvent_Event_0)))
    (:then_2
      (bind _returnvalue (Animation|GetPlayLength (Utilities|Array|Get(acopy) (Variables|애니메이션|GetAttackJumpAnimMontage) 1)))
      (Variables|Default|SetJumpingTime _returnvalue)
      (Variables|Default|SetJumpAttackAxisCurve "/Game/Hyun_BossCharacter/Curves/JumpChaseAttackCurve.JumpChaseAttackCurve")
      (Utilities|Array|AddUnique _cables (Variables|Default|Get1))
      (Utilities|Array|AddUnique _cables (Variables|Default|Get2))
      (Utilities|Array|AddUnique _cables (Variables|Default|Get3))
      (Utilities|Array|AddUnique _cables (Variables|Default|Get4)))
    (:then_3
      (EventDispatchers|AssignOnDeadEvent (delegate Custom|OnDeadEvent_Event_0)))))

(event EventTick
  (params (DeltaSeconds :type Float%20%28single-precision%29))
  (Utilities|FlowControl|Sequence
    (:then_0
      (Utilities|FlowControl|Delay 1.8)
      (Variables|Default|SetHealth (Math|Integer|Min(Integer) (+ (Variables|Default|GetHealth) 1) (Variables|Default|GetMaxHealth))))))

(fn ConstructionScript)

(fn OnPlayMontage
  (params (MontageName :type Name) (AnimTime :type Float%20%28single-precision%29))
  (bind _animmontages (Variables|디폴트|GetAnimMontages))
  (bind (_value _returnvalue) (Utilities|Map|Find _animmontages MontageName))
  (if _returnvalue
    (CallFunction|OnPlayAnimMontage _value AnimTime)))

(fn AddMontage
  (params (MontageName :type Name) (Montage :type Anim%20Montage%20Object%20Reference))
  (bind _animmontages (Variables|디폴트|GetAnimMontages))
  (if (not (Utilities|Map|Contains _animmontages MontageName))
    (Utilities|Map|Add _animmontages MontageName Montage)))

(fn AddMontageList
  (params (MontageName :type Name) (Montages :type Array%20of%20Anim%20Montage%20Object%20References))
  (for (_array_element _array_index) Montages
    (CallFunction|AddMontage (Utilities|String|StringToName (Utilities|String|BuildString(Name) "" "" MontageName (Utilities|String|ToString(Integer) _array_index))) _array_element)))

(fn OnLog
  (params (actionType :type Integer))
  (Development|PrintString (Utilities|String|BuildString(Name) "" "" "Boss : " (Utilities|String|EnumtoString (Utilities|Enum|ByteToEnumEBossAction (Math|Conversions|ToByte(Integer) actionType))))))

(fn OnShoot
  (bind _returnvalue (Game|SpawnActorfromClass (Variables|Default|GetProjectile) (Transformation|GetActorTransform) "Undefined" 0 0))
  (Utilities|IsValid _returnvalue))

(fn OnCoreBroke
  (params (Index :type Integer))
  (bind _returnvalue (+ Index 1))
  (Utilities|IsValid (Utilities|Array|Get(acopy) (Variables|Default|GetCables) Index)
    (:Is%20Valid
      (bind _returnvalue_2 (Rendering|Material|CreateDynamicMaterialInstance (Variables|Character|GetMesh) 4 "/Game/Hyun_BossCharacter/Mesh/Materials/MI_Hetto_boss_thread.MI_Hetto_boss_thread" "None" :!class /Script/Engine.PrimitiveComponent))
      (Rendering|Material|SetScalarParameterValue _returnvalue_2 (Utilities|String|StringToName (Utilities|String|BuildString(Integer) "" "Thread_C_0" _returnvalue)) 1.0 :!class /Script/Engine.MaterialInstanceDynamic)
      (Development|PrintString (Utilities|String|BuildString(Name) "" "" "CoreBroke STart" (Utilities|String|ToString(Integer) _returnvalue))))))