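; BP_BossCharacterProjectile is a boss projectile actor that travels straight up along world Z at very high speed.
; Each Tick it moves with a swept SetActorLocation scaled by delta time and destroys itself on a blocking hit.
; A disconnected, zero-length line trace would call OnHit with fixed damage, but it never runs, so the projectile applies no damage in this graph.
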(event EventTick
  (params (DeltaSeconds :type Float%20%28single-precision%29))
  (bind _sweephitresult (Transformation|SetActorLocation (+ (Transformation|GetActorLocation) (Math|Vector|MakeVector 0.0 0.0 (* DeltaSeconds 1e+03 5e+01))) true false))
  (if (.bBlockingHit (Collision|BreakHitResult _sweephitresult))
    (Utilities|FlowControl|Sequence
      (:then_1
        (Actor|DestroyActor)))))

(fn ConstructionScript)