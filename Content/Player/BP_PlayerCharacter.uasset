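; Player character Blueprint for sword-and-gun combat, handling montages, projectile shots, gun-counter camera changes, state-based damage shakes and pause input.
; BeginPlay builds a name-to-montage map with index-suffixed variants, loads saved mouse sensitivity and grows the sensing sphere by timeline.
; OnPlayMontage plays montages by name and forwards their callbacks, as sensing overlaps are forwarded to eye-sense handlers.
; Gun-counter events set camera arm and FOV directly, leaving their blend timelines and slow-motion timeline disconnected.
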(event Custom|InitalizedAnimation
  (Utilities|FlowControl|Sequence
    (:then_0
      (CallFunction|AddMontage (Variables|Default|GetAnimMontageNameDash) (Variables|AnimMontage|GetDashAnimMontage))
      (CallFunction|AddMontage (Variables|Default|GetAnimMontageNameHit) (Variables|AnimMontage|GetHitAnimMontage))
      (CallFunction|AddMontage (Variables|Default|GetAnimMontageNameDead) (Variables|AnimMontage|GetDeadAnimMontage))
      (CallFunction|AddMontage (Variables|Default|GetAnimMontageNameKnockdown) (Variables|AnimMontage|GetKnockdownAnimMontage))
      (CallFunction|AddMontage (Variables|Default|GetAnimMontageNameRise) (Variables|AnimMontage|GetRiseAnimMontage))
      (CallFunction|AddMontage (Variables|Default|GetAnimMontageNameSwordCounter) (Variables|AnimMontage|GetSwordCounterAttackAnimMontage)))
    (:then_1
      (CallFunction|InitMontageList (Variables|AnimMontage|GetAttackStartAnimMontages) (Variables|Default|GetAnimMontageNameAttackStart))
      (CallFunction|InitMontageList (Variables|AnimMontage|GetDefaultAttackAnimMontages) (Variables|Default|GetAnimMontageNameDefaultAttack))
      (CallFunction|InitMontageList (Variables|AnimMontage|GetStrongAttackAnimMontages) (Variables|Default|GetAnimMontageNameStrongAttack))
      (CallFunction|InitMontageList (Variables|AnimMontage|GetAttackFailAnimMontages) (Variables|Default|GetAnimMontageNameAttackFail))
      (CallFunction|InitMontageList (Variables|AnimMontage|GetGunCounterAttackAnimMontages) (Variables|Default|GetAnimMontageNameGunCounter))
      (CallFunction|InitMontageList (Variables|AnimMontage|GetBlockAnimMontages) (Variables|Default|GetAnimMontageNameBlock))
      (CallFunction|InitMontageList (Variables|AnimMontage|GetRiseDashAnimMontage) (Variables|Default|GetAnimMontageNameRiseDash)))))

(event Custom|OnGunCounterStartEvent_Event_0
  (bind _cameramanager (Variables|Default|GetCameraManager))
  (bind _maincameraarm (Variables|Default|GetMainCameraArm))
  (Variables|/Script/Engine.SpringArmComponent|SetTargetArmLength _maincameraarm (Math|Float|Lerp (Variables|/Script/Engine.SpringArmComponent|GetTargetArmLength _maincameraarm) 3e+02 (stale _duration)))
  (Variables|/Script/Engine.SpringArmComponent|SetSocketOffset _maincameraarm (Math|Vector|MakeVector 0.0 (Math|Float|Lerp (.y (Variables|/Script/Engine.SpringArmComponent|GetSocketOffset _maincameraarm)) 8e+01 (stale _duration)) (Math|Float|Lerp (.z (Variables|/Script/Engine.SpringArmComponent|GetSocketOffset _maincameraarm)) 5.0 (stale _duration))))
  (Variables|/Script/Engine.SpringArmComponent|SetCameraLagSpeed _maincameraarm (Math|Float|Lerp (Variables|/Script/Engine.SpringArmComponent|GetCameraLagSpeed _maincameraarm) 0.0 (stale _duration)))
  (Variables|/Script/Engine.SpringArmComponent|SetCameraRotationLagSpeed _maincameraarm (Math|Float|Lerp (Variables|/Script/Engine.SpringArmComponent|GetCameraRotationLagSpeed _maincameraarm) 0.0 (stale _duration)))
  (Variables|/Script/Engine.CameraComponent|SetFieldOfView _cameramanager (Math|Float|Lerp (Variables|/Script/Engine.CameraComponent|GetFieldOfView _cameramanager) 7e+01 (stale _duration))))

(event Custom|OnGunCounterEndEvent_Event_0
  (bind _maincameraarm (Variables|Default|GetMainCameraArm))
  (Variables|/Script/Engine.SpringArmComponent|SetTargetArmLength _maincameraarm 4e+02)
  (Variables|/Script/Engine.SpringArmComponent|SetSocketOffset _maincameraarm (Math|Vector|MakeVector 0.0 0.0 0.0))
  (Variables|/Script/Engine.SpringArmComponent|SetCameraLagSpeed _maincameraarm 1e+01)
  (Variables|/Script/Engine.SpringArmComponent|SetCameraRotationLagSpeed _maincameraarm 3e+01)
  (Variables|/Script/Engine.CameraComponent|SetFieldOfView (Variables|Default|GetCameraManager) 75.0))

(event Custom|OnShootEvent_1
  (params (EndLocation :type Vector%20%28by%20ref%29))
  (bind _returnvalue (Game|SpawnActorfromClass "/Game/Player/BP_PlayerProjectile.BP_PlayerProjectile_C" (Math|Transform|MakeTransform (Transformation|GetSocketLocation (Variables|Character|GetMesh) (Variables|Default|GetGunMuzzleEffectPoint)) (Transformation|GetWorldRotation (Variables|Default|GetMainCameraArm)) "1,1,1") "Undefined" 0 0))
  (Default|Shoot _returnvalue EndLocation "/Game/FX/PC/15_Gun_ShootHit/FX_PC_Gun_ShootHit.FX_PC_Gun_ShootHit"))

(event EventBeginPlay
  (Utilities|FlowControl|Sequence
    (:then_0
      (CallFunction|InitalizedAnimation)
      (|InitEyeSensing
        (:Exit
          (bind _returnvalue (SaveGame|DoesSaveGameExist (Variables|Default|GetSaveFileName)))
          (if _returnvalue
            (bind _returnvalue_2 (SaveGame|LoadGamefromSlot (Variables|Default|GetSaveFileName)))
            (bind _asbp_save_game (Utilities|Casting|CastToBP_SaveGame _returnvalue_2))
            (Variables|Default|SetMouseSensitivity (.mousesensitivity (.optiondata (Variables|/Game/Player/Save/BP_SaveGame.BP_SaveGame_C|GetData _asbp_save_game))))))))
    (:then_1
      (bind _linearvalue (Timeline|SensingInitialized PlayFromStart)
        (:Update
          (Components|Sphere|SetSphereRadius (Variables|Default|GetSensingCollision) (Math|Float|Lerp 0.0 1.5e+03 _linearvalue) true))))
    (:then_2
      (EventDispatchers|AssignOnShootEvent (delegate Custom|OnShootEvent_1))
      (EventDispatchers|AssignOnGunCounterStartEvent (delegate Custom|OnGunCounterStartEvent_Event_0))
      (EventDispatchers|AssignOnGunCounterEndEvent (delegate Custom|OnGunCounterEndEvent_Event_0)))))

(event Game|Damage|EventPointDamage
  (params (Damage :type Float%20%28single-precision%29) (DamageType :type Damage%20Type%20Object%20Reference) (HitLocation :type Vector :default "0, 0, 0") (HitNormal :type Vector :default "0, 0, 0") (HitComponent :type Primitive%20Component%20Object%20Reference) (BoneName :type Name :default "None") (ShotFromDirection :type Vector :default "0, 0, 0") (InstigatedBy :type Controller%20Object%20Reference) (DamageCauser :type Actor%20Object%20Reference) (HitInfo :type Hit%20Result%20Structure%20%28by%20ref%29))
  (switch Utilities|FlowControl|Switch|SwitchonEPlayerState (Variables|Default|GetCurState)
    (:Idle
      (if true :!label _label
        (Camera|PlayWorldCameraShake "/Game/Player/Camera/CamShake_Hit.CamShake_Hit_C" (Transformation|GetActorLocation) 0.0 5e+02)))
    (:Hit
      (goto _label))
    (:Block
      (if true
        (Camera|PlayWorldCameraShake "/Game/Player/Camera/CamShake_Block.CamShake_Block_C" (Transformation|GetActorLocation) 0.0 5e+02)))
    (:Parry
      (if true
        (Camera|PlayWorldCameraShake "/Game/Player/Camera/CamShake_Parry.CamShake_Parry_C" (Transformation|GetActorLocation) 0.0 5e+02)))))

(event Input|ActionEvents|InputActionEscape
  (params (Key :type Key%20Structure :default "None"))
  (bind _hud (Variables|Default|GetHUD))
  (:Pressed
    (Utilities|IsValid (Variables|Default|GetHUD)
      (:Is%20Valid
        (if (Game|IsGamePaused)
          (Default|Resume _hud)
          (else
            (Default|Pause _hud)))))))

(fn ConstructionScript)

(fn OnPlayMontage
  (params (MontageName :type Name) (AnimTime :type Float%20%28single-precision%29))
  (bind _animmontagelist (Variables|DataTable|GetAnimMontageList))
  (bind (_value _returnvalue) (Utilities|Map|Find _animmontagelist MontageName))
  (if _returnvalue
    (CallFunction|OnPlayAnimMontage _value AnimTime)))

(fn AddMontage
  (params (MontageName :type Name) (Montage :type Anim%20Montage%20Object%20Reference))
  (bind _animmontagelist (Variables|DataTable|GetAnimMontageList))
  (if (not (Utilities|Map|Contains _animmontagelist MontageName))
    (Utilities|Map|Add _animmontagelist MontageName Montage)))

(fn OnLog
  (params (State :type Integer)))

(fn OnLogString
  (params (String :type String)))

(event OnComponentBeginOverlap(SensingCollision)
  (params (OverlappedComponent :type Primitive%20Component%20Object%20Reference) (OtherActor :type Actor%20Object%20Reference) (OtherComp :type Primitive%20Component%20Object%20Reference) (OtherBodyIndex :type Integer) (bFromSweep :type Boolean) (SweepResult :type Hit%20Result%20Structure%20%28by%20ref%29))
  (Class|PlayerCharacter|OnEyeSenseEnter OverlappedComponent OtherActor OtherComp OtherBodyIndex bFromSweep SweepResult))

(event OnComponentEndOverlap(SensingCollision)
  (params (OverlappedComponent :type Primitive%20Component%20Object%20Reference) (OtherActor :type Actor%20Object%20Reference) (OtherComp :type Primitive%20Component%20Object%20Reference) (OtherBodyIndex :type Integer))
  (Class|PlayerCharacter|OnEyeSenseExit OverlappedComponent OtherActor OtherComp OtherBodyIndex))

(event Custom|InitMontageList
  (params (Montage :type Array%20of%20Anim%20Montage%20Object%20References) (MontageName :type Name))
  (for (_array_element _array_index) Montage
    (CallFunction|AddMontage (Utilities|String|StringToName (Utilities|String|BuildString(Name) "" "" MontageName (Utilities|String|ToString(Integer) _array_index))) _array_element)))

(event Custom|OnPlayAnimMontage
  (params (PlayMontage :type Anim%20Montage%20Object%20Reference) (StartPosition :type Float%20%28single-precision%29))
  (bind _notifyname (Animation|Montage|PlayMontage (Variables|Character|GetMesh) PlayMontage 1.0 StartPosition)
    (:OnCompleted
      (Class|CharacterMaster|OnAnimCompleted))
    (:OnBlendOut
      (Class|CharacterMaster|OnAnimBlendOut))
    (:OnInterrupted
      (Class|CharacterMaster|OnAnimInterrupted))
    (:OnNotifyBegin
      (Class|CharacterMaster|OnAnimNotifyBegin _notifyname))))