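; Player character Blueprint handling Escape pause menu, saved mouse sensitivity, montage playback and damage camera shakes chosen by current state.
; On BeginPlay it registers montages in a name-keyed map, suffixing array entries with their index.
; Name lookups play these montages, forwarding completion, blend-out, interrupt and notify callbacks to handler functions.
; A timeline grows the sensing sphere at startup, and its overlaps feed eye-sense enter and exit handlers.
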(event Custom|InitalizedAnimation
  (Utilities|FlowControl|Sequence
    (:then_0
      (CallFunction|AddMontage (Variables|Default|GetAnimMontageNameDash) (Variables|AnimMontage|GetDashAnimMontage))
      (CallFunction|AddMontage (Variables|Default|GetAnimMontageNameHit) (Variables|AnimMontage|GetHitAnimMontage))
      (CallFunction|AddMontage (Variables|Default|GetAnimMontageNameDead) (Variables|AnimMontage|GetDeadAnimMontage))
      (CallFunction|AddMontage (Variables|Default|GetAnimMontageNameKnockdown) (Variables|AnimMontage|GetKnockdownAnimMontage))
      (CallFunction|AddMontage (Variables|Default|GetAnimMontageNameRise) (Variables|AnimMontage|GetRiseAnimMontage))
      (CallFunction|AddMontage (Variables|Default|GetAnimMontageNameRiseDash) (Variables|AnimMontage|GetRiseDashAnimMontage))
      (CallFunction|AddMontage (Variables|Default|GetAnimMontageNameSwordCounter) (Variables|AnimMontage|GetSwordCounterAttackAnimMontage)))
    (:then_1
      (CallFunction|InitMontageList (Variables|AnimMontage|GetAttackStartAnimMontages) (Variables|Default|GetAnimMontageNameAttackStart))
      (CallFunction|InitMontageList (Variables|AnimMontage|GetDefaultAttackAnimMontages) (Variables|Default|GetAnimMontageNameDefaultAttack))
      (CallFunction|InitMontageList (Variables|AnimMontage|GetStrongAttackAnimMontages) (Variables|Default|GetAnimMontageNameStrongAttack))
      (CallFunction|InitMontageList (Variables|AnimMontage|GetAttackFailAnimMontages) (Variables|Default|GetAnimMontageNameAttackFail))
      (CallFunction|InitMontageList (Variables|AnimMontage|GetGunCounterAttackAnimMontages) (Variables|Default|GetAnimMontageNameGunCounter))
      (CallFunction|InitMontageList (Variables|AnimMontage|GetBlockAnimMontages) (Variables|Default|GetAnimMontageNameBlock)))))

(event EventBeginPlay
  (Utilities|FlowControl|Sequence
    (:then_0
      (CallFunction|InitalizedAnimation)
      (|InitEyeSensing
        (:Exit
          (bind _returnvalue (SaveGame|DoesSaveGameExist (Variables|Default|GetSaveFileName)))
          (if _returnvalue
            (bind _returnvalue_2 (SaveGame|LoadGamefromSlot (Variables|Default|GetSaveFileName)))
            (bind _asbp_save_game (Utilities|Casting|CastToBP_SaveGame _returnvalue_2))
            (Variables|Default|SetMouseSensitivity (.mousesensitivity (.optiondata (Variables|/Game/Player/Save/BP_SaveGame.BP_SaveGame_C|GetData _asbp_save_game))))))))
    (:then_1
      (bind _linearvalue (Timeline|SensingInitialized PlayFromStart)
        (:Update
          (Components|Sphere|SetSphereRadius (Variables|Default|GetSensingCollision) (Math|Float|Lerp 0.0 1.5e+03 _linearvalue) true))))
    (:then_2
      (bind _returnvalue_3 (UserInterface|CreateWidget "/Game/UMG/PauseWidget.PauseWidget_C"))
      (bind _output_get (Variables|Default|SetPauseWidget _returnvalue_3))
      (UserInterface|Viewport|AddtoViewport _output_get 0)
      (Widget|SetVisibility _output_get "Collapsed"))))

(event Game|Damage|EventPointDamage
  (params (Damage :type Float%20%28single-precision%29) (DamageType :type Damage%20Type%20Object%20Reference) (HitLocation :type Vector :default "0, 0, 0") (HitNormal :type Vector :default "0, 0, 0") (HitComponent :type Primitive%20Component%20Object%20Reference) (BoneName :type Name :default "None") (ShotFromDirection :type Vector :default "0, 0, 0") (InstigatedBy :type Controller%20Object%20Reference) (DamageCauser :type Actor%20Object%20Reference) (HitInfo :type Hit%20Result%20Structure%20%28by%20ref%29))
  (switch Utilities|FlowControl|Switch|SwitchonEPlayerState (Variables|Default|GetCurState)
    (:Idle
      (if true :!label _label
        (Camera|PlayWorldCameraShake "/Game/Player/Camera/CamShake_Hit.CamShake_Hit_C" (Transformation|GetActorLocation) 0.0 5e+02)))
    (:Hit
      (goto _label))
    (:Parry
      (if true
        (Camera|PlayWorldCameraShake "/Game/Player/Camera/CamShake_Parry.CamShake_Parry_C" (Transformation|GetActorLocation) 0.0 5e+02)))))

(event Input|ActionEvents|InputActionEscape
  (params (Key :type Key%20Structure))
  (:Pressed
    (Utilities|IsValid (Variables|Default|GetPauseWidget)
      (:Is%20Valid
        (if (Game|IsGamePaused)
          (CallFunction|OnGameResume)
          (else
            (CallFunction|OnGamePause)))))))

(fn ConstructionScript)

(fn OnPlayMontage
  (params (MontageName :type Name) (AnimTime :type Float%20%28single-precision%29))
  (bind _animmontagelist (Variables|DataTable|GetAnimMontageList))
  (bind (_value _returnvalue) (Utilities|Map|Find _animmontagelist MontageName))
  (if _returnvalue
    (CallFunction|OnPlayAnimMontage _value AnimTime)))

(fn AddMontage
  (params (MontageName :type Name) (Montage :type Anim%20Montage%20Object%20Reference))
  (bind _animmontagelist (Variables|DataTable|GetAnimMontageList))
  (if (not (Utilities|Map|Contains _animmontagelist MontageName))
    (Utilities|Map|Add _animmontagelist MontageName Montage)))

(fn OnLog
  (params (State :type Integer))
  (Development|PrintString (Utilities|String|BuildString(Name) "" "" "Player : " (Utilities|String|EnumtoString (Utilities|Enum|ByteToEnumEPlayerState (Math|Conversions|ToByte(Integer) State))))))

(fn OnLogString
  (params (String :type String))
  (Development|PrintString (Utilities|String|BuildString(Name) "" "" "Player : " String)))

(fn OnGameResume
  (bind _pausewidget (Variables|Default|GetPauseWidget))
  (Utilities|IsValid _pausewidget
    (:Is%20Valid
      (Game|SetGamePaused false)
      (Widget|SetVisibility _pausewidget "Collapsed")
      (Variables|/Script/Engine.PlayerController|SetbShowMouseCursor (Game|GetPlayerController 0) false))))

(fn OnGamePause
  (Utilities|IsValid (Variables|Default|GetPauseWidget)
    (:Is%20Valid
      (Game|SetGamePaused true)
      (Widget|SetVisibility (Variables|Default|GetPauseWidget) "Visible")
      (Variables|/Script/Engine.PlayerController|SetbShowMouseCursor (Game|GetPlayerController 0) true))))

(event OnComponentBeginOverlap(SensingCollision)
  (params (OverlappedComponent :type Primitive%20Component%20Object%20Reference) (OtherActor :type Actor%20Object%20Reference) (OtherComp :type Primitive%20Component%20Object%20Reference) (OtherBodyIndex :type Integer) (bFromSweep :type Boolean) (SweepResult :type Hit%20Result%20Structure%20%28by%20ref%29))
  (Class|PlayerCharacter|OnEyeSenseEnter OverlappedComponent OtherActor OtherComp OtherBodyIndex bFromSweep SweepResult))

(event OnComponentEndOverlap(SensingCollision)
  (params (OverlappedComponent :type Primitive%20Component%20Object%20Reference) (OtherActor :type Actor%20Object%20Reference) (OtherComp :type Primitive%20Component%20Object%20Reference) (OtherBodyIndex :type Integer))
  (Class|PlayerCharacter|OnEyeSenseExit OverlappedComponent OtherActor OtherComp OtherBodyIndex))

(event Custom|InitMontageList
  (params (Montage :type Array%20of%20Anim%20Montage%20Object%20References) (MontageName :type Name))
  (for (_array_element _array_index) Montage
    (CallFunction|AddMontage (Utilities|String|StringToName (Utilities|String|BuildString(Name) "" "" MontageName (Utilities|String|ToString(Integer) _array_index))) _array_element)))

(event Custom|OnPlayAnimMontage
  (params (PlayMontage :type Anim%20Montage%20Object%20Reference) (StartPosition :type Float%20%28single-precision%29))
  (bind _notifyname (Animation|Montage|PlayMontage (Variables|Character|GetMesh) PlayMontage 1.0 StartPosition)
    (:OnCompleted
      (Class|CharacterMaster|OnAnimCompleted))
    (:OnBlendOut
      (Class|CharacterMaster|OnAnimBlendOut))
    (:OnInterrupted
      (Class|CharacterMaster|OnAnimInterrupted))
    (:OnNotifyBegin
      (Class|CharacterMaster|OnAnimNotifyBegin _notifyname))))