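; Player projectile Blueprint that acts as a visible gun shot traveling to a given impact point, with a trail effect hidden until Shoot is called.
; Shoot plays the Duration timeline, lerping from the current location, not a stored start, toward the impact point with sweep.
; When the timeline finishes, it hides the trail and destroys the actor, guarded by IsShoot.
; The blocking-hit branch does nothing; impact emitter and early-destroy logic are disconnected.
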(event Custom|Shoot
  (params (ImpactPoint :type Vector) (Effect :type Particle%20System%20Object%20Reference))
  (Rendering|SetVisibility (Variables|Default|GetFX_PC_Gun_Trail) true false)
  (Variables|Default|SetIsShoot false)
  (bind _duration (Timeline|Duration PlayFromStart)
    (:Update
      (bind _sweephitresult (Transformation|SetActorLocation (Math|Vector|Lerp(Vector) (Transformation|GetActorLocation) ImpactPoint _duration) true false))
      (if (.bBlockingHit (Collision|BreakHitResult _sweephitresult))
        _))
    (:Finished
      (if (not (Variables|Default|GetIsShoot))
        (Variables|Default|SetIsShoot true)
        (Rendering|SetVisibility (Variables|Default|GetFX_PC_Gun_Trail) false false)
        (Actor|DestroyActor)))))

(event EventBeginPlay
  (Rendering|SetVisibility (Variables|Default|GetFX_PC_Gun_Trail) false false))

(fn ConstructionScript)