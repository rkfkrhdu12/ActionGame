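; Monster AI state for a rush attack that charges at the player and then plays an end-of-attack montage.
; On enable it stops movement, then after a short delay quadruples walk speed and starts a looping timer.
; Each loop tick moves toward the player until close, then clears the timer, plays the montage and switches to Observe.
; Disabling the state restores default walk speed.
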(event Custom|StartRush
  ;[0.15 0.15 0.15 0.5] Single - StartRush()
  (bind _returnvalue (Class|UserdefinedState|IsValidTimer (stale EventOnEnable _timerhandle)))
  (if _returnvalue
    (Variables|/Script/Engine.CharacterMovementComponent|SetMaxWalkSpeed (Variables|/Script/Engine.Character|GetCharacterMovement (Variables|Default|GetMyCharacter)) (* (Variables|Default|GetDefaultWalkSpeed) 4.0))
    (bind _timerhandle (Class|UserdefinedState|StartDelay 0.1 true))
    (Variables|Default|SetRushLoopTimerHandle _timerhandle)))

(event Custom|LoopRush
  ;[0.15 0.15 0.15 0.5] Loop - LoopRush()
  (bind _returnvalue (Class|UserdefinedState|IsValidTimer (Variables|Default|GetRushLoopTimerHandle)))
  (if _returnvalue
    (if (> (Class|UserdefinedMonsterState|GetDistancetoPlayer) 3.5e+02)
      (Class|UserdefinedMonsterState|OnMovetoLocation (Class|UserdefinedMonsterState|GetPlayerLocation))
      (else
        (Class|UserdefinedState|ClearTimer (Variables|Default|GetRushLoopTimerHandle))
        (Animation|Montage|PlayMontage (Variables|Default|GetMyMesh) "/Game/Hyun_BossCharacter/Animations/Hetto_RushAttack_End_Montage.Hetto_RushAttack_End_Montage"
          (:OnCompleted
            (Class|CharacterBase|ChangeState (Variables|Default|GetMyMonsterCharacter) "/Game/Project/Blueprints/Monster/FMonsterState.FMonsterState" "Observe")))))))

(event EventOnEnable
  ;[0.15 0.15 0.15 0.5] OnEnable
  (AI|Navigation|StopMovement (Variables|Default|GetMyAIController))
  (bind _timerhandle (Class|UserdefinedState|StartDelay 0.1)))

(event EventOnDisable
  ;[0.15 0.15 0.15 0.5] OnDisable
  (Variables|/Script/Engine.CharacterMovementComponent|SetMaxWalkSpeed (Variables|/Script/Engine.Character|GetCharacterMovement (Variables|Default|GetMyCharacter)) (Variables|Default|GetDefaultWalkSpeed)))

(event EventOnDelayFinished
  ;[0.15 0.15 0.15 0.5] OnDelayFinished
  (Utilities|FlowControl|Sequence
    (:then_0
      (CallFunction|StartRush))
    (:then_1
      (CallFunction|LoopRush))))