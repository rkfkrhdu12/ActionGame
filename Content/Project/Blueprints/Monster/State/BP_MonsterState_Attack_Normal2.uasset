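; Monster state for a second normal attack, a melee combo by the Hetto monster that runs when the state is enabled.
; CheckDistanceToPlayer stores a fixed attack range on the monster character and compares it with the player's distance, switching to Chase when out of range.
; In range, the basic attack montage chains into the strong one on blend out, then switches to Dodge on completion.
; A random AttackType is rolled, but its switch is unconnected.
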(event EventOnEnable
  (Utilities|FlowControl|Sequence
    (:then_0
      (Utilities|CheckDistancetoPlayer 3e+02
        (:Success
          (Animation|Montage|PlayMontage (Variables|Default|GetMyMesh) "/Game/Hyun_BossCharacter/Animations/Hetto_Attack01_Montage.Hetto_Attack01_Montage"
            (:OnBlendOut
              (Animation|Montage|PlayMontage (Variables|Default|GetMyMesh) "/Game/Hyun_BossCharacter/Animations/Hetto_Attack01Strong_Montage.Hetto_Attack01Strong_Montage"
                (:OnCompleted
                  (Class|UserdefinedState|ChangeState "/Game/Project/Blueprints/Monster/FMonsterState.FMonsterState" "Dodge"))))))
        (:Failed
          (Class|UserdefinedState|ChangeState "/Game/Project/Blueprints/Monster/FMonsterState.FMonsterState" "Chase"))))
    (:then_1
      (Variables|Default|SetAttackType (Math|Integer|%(Integer) (Math|Random|RandomInteger 100) (Variables|Default|GetAttackTypeCount))))))