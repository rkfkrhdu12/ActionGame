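; Monster chase state that runs toward the player at boosted walk speed, restoring the default when disabled.
; A short looping timer refreshes the move target and switches to AttackNormal once the player is within the monster's attack distance.
; A one-shot timer instead picks AttackRush or AttackJump by player distance.
; Both timers share one delay-finished event, with each branch gated by its timer handle.
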(event Custom|LoopChase
  ;[0.15 0.15 0.15 0.5] Loop - LoopChase()
  (bind _returnvalue (Class|UserdefinedState|IsValidTimer (Variables|Default|GetLoopTimer%20Handle)))
  (if _returnvalue
    (bind _asbp_monster_character (Utilities|Casting|CastToBP_MonsterCharacter (Variables|Default|GetMyMonsterCharacter)))
    (if (< (Class|UserdefinedMonsterState|GetDistancetoPlayer) (Variables|/Game/Project/Blueprints/Monster/BP_MonsterCharacter.BP_MonsterCharacter_C|GetAttackDistance _asbp_monster_character))
      (Class|CharacterBase|ChangeState (Variables|Default|GetMyMonsterCharacter) "/Game/Project/Blueprints/Monster/FMonsterState.FMonsterState" "AttackNormal")
      (Class|UserdefinedState|ClearTimer (Variables|Default|GetLoopTimer%20Handle))
      (else
        (Class|UserdefinedMonsterState|OnMovetoLocation (Class|UserdefinedMonsterState|GetPlayerLocation))))))

(event Custom|NextAttackChanged
  (bind _returnvalue (Class|UserdefinedMonsterState|GetDistancetoPlayer))
  ;[0.15 0.15 0.15 0.5] Single - NextAttackChanged()
  (bind _returnvalue_2 (Class|UserdefinedState|IsValidTimer (stale EventOnEnable _timerhandle_2)))
  (if _returnvalue_2
    (Development|PrintString 0 (Utilities|String|ToString(Float) _returnvalue))
    (if (> _returnvalue 1e+03)
      (Class|CharacterBase|ChangeState (Variables|Default|GetMyMonsterCharacter) "/Game/Project/Blueprints/Monster/FMonsterState.FMonsterState" "AttackRush")
      (Class|UserdefinedState|ClearTimer (Variables|Default|GetLoopTimer%20Handle))
      (else
        (Class|CharacterBase|ChangeState (Variables|Default|GetMyMonsterCharacter) "/Game/Project/Blueprints/Monster/FMonsterState.FMonsterState" "AttackJump")
        (Class|UserdefinedState|ClearTimer (Variables|Default|GetLoopTimer%20Handle))))))

(event EventOnDelayFinished
  ;[0.15 0.15 0.15 0.5] OnDealyFinished
  (Utilities|FlowControl|Sequence
    (:then_0
      (CallFunction|LoopChase))
    (:then_1
      (CallFunction|NextAttackChanged))))

(event EventOnEnable
  ;[0.15 0.15 0.15 0.5] OnEnable
  (Variables|/Script/Engine.CharacterMovementComponent|SetMaxWalkSpeed (Variables|/Script/Engine.Character|GetCharacterMovement (Variables|Default|GetMyCharacter)) (* (Variables|Default|GetDefaultWalkSpeed) 1.5))
  (bind _timerhandle (Class|UserdefinedState|StartDelay 0.3 true))
  (Variables|Default|SetLoopTimer%20Handle _timerhandle)
  (bind _timerhandle_2 (Class|UserdefinedState|StartDelay 2.0))
  (Class|UserdefinedMonsterState|OnMovetoLocation (Class|UserdefinedMonsterState|GetPlayerLocation)))

(event EventOnDisable
  ;[0.15 0.15 0.15 0.5] OnDisable
  (Variables|/Script/Engine.CharacterMovementComponent|SetMaxWalkSpeed (Variables|/Script/Engine.Character|GetCharacterMovement (Variables|Default|GetMyCharacter)) (Variables|Default|GetDefaultWalkSpeed)))