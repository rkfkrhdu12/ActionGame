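; Monster AI state for patrolling, which wanders between random points until a short start delay hands over to the Observe state.
; On enable it compares player distance to a threshold and always makes its first move to a random point around the player.
; Each finished move picks another point, around the monster if the player was far, otherwise in a wider radius around the player.
; A deprecated line-trace fan detection and an attack montage call remain unconnected.
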(event Custom|NextStateTimerEvent
  (bind _returnvalue (Class|UserdefinedState|IsValidTimer (stale EventOnEnable _timerhandle)))
  (if _returnvalue
    (Class|CharacterBase|ChangeState (Variables|Default|GetMyCharacter) "/Game/Project/Blueprints/Monster/FMonsterState.FMonsterState" "Observe")))

(event EventOnEnable
  (Variables|Default|SetbIsDefaultPatrolType (< (Variables|OnEnable|GetCheckDistanceToPlayer) (Math|Vector|Distance(Vector) (Class|UserdefinedMonsterState|GetPlayerLocation) (Class|UserdefinedState|GetActorLocation))) :!pinned true) ; Check Distance to Player (패턴의 기준이 되는 거리)\n보다 멀면 True (기본 형태로 순찰) \n보다 가까우면 False (플레이어 위치 주변으로 순찰)
  (Class|UserdefinedMonsterState|OnMoveRandomPointinRadius (Class|UserdefinedMonsterState|GetPlayerLocation) 2e+03)
  (bind _timerhandle (Class|UserdefinedState|StartDelay 3.0)))

(event EventOnMoveFinished
  (params (bIsSuccess :type Boolean))
  (if (Variables|Default|GetbIsDefaultPatrolType)
    (Class|UserdefinedMonsterState|OnMoveRandomPointinRadius (Class|UserdefinedState|GetActorLocation) 1e+03)
    (else
      (Class|UserdefinedMonsterState|OnMoveRandomPointinRadius (Class|UserdefinedMonsterState|GetPlayerLocation) 2e+03))))

(event EventOnDelayFinished
  (CallFunction|NextStateTimerEvent))

(event EventTick
  (params (DeltaTime :type Float%20%28single-precision%29)))