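; Normal attack state for a monster, which runs one of three Hetto melee montage patterns against the player.
; On enable it faces the player and branches on AttackType, rerolling unrecognized values.
; DistanceToPlayer stores the attack range on the monster character and gates each pattern, switching to Chase when out of range.
; One pattern chains two montages on blend out; finished attacks switch to Dodge and randomize the next AttackType.
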(event EventOnEnable
  (CallFunction|LookatPlayer)
  (switch int (Variables|Default|GetAttack%20Type) :!label _label
    (:Default
      (Variables|Default|SetAttack%20Type (Math|Random|RandomInteger 2))
      (goto _label))
    (:0
      (Utilities|DistancetoPlayer 3e+02
        (:Success
          (Animation|Montage|PlayMontage (Variables|Default|GetMyMesh) "/Game/Hyun_BossCharacter/Animations/Hetto_Attack01_Montage.Hetto_Attack01_Montage"
            (:OnBlendOut
              (Animation|Montage|PlayMontage (Variables|Default|GetMyMesh) "/Game/Hyun_BossCharacter/Animations/Hetto_Attack01Strong_Montage.Hetto_Attack01Strong_Montage"
                (:OnCompleted
                  (Class|CharacterBase|ChangeState (Variables|Default|GetMyCharacter) "/Game/Project/Blueprints/Monster/FMonsterState.FMonsterState" "Dodge")
                  (Variables|Default|SetAttack%20Type (Math|Integer|%(Integer) (Math|Random|RandomInteger 10) 3) :!label _label_2))))))
        (:Fail
          (Class|CharacterBase|ChangeState (Variables|Default|GetMyCharacter) "/Game/Project/Blueprints/Monster/FMonsterState.FMonsterState" "Chase"))))
    (:1
      (Utilities|DistancetoPlayer 3e+02
        (:Success
          (Animation|Montage|PlayMontage (Variables|Default|GetMyMesh) "/Game/Hyun_BossCharacter/Animations/Hetto_AttackNormal_Montage.Hetto_AttackNormal_Montage"
            (:OnCompleted
              (Class|CharacterBase|ChangeState (Variables|Default|GetMyCharacter) "/Game/Project/Blueprints/Monster/FMonsterState.FMonsterState" "Dodge")
              (goto _label_2))))
        (:Fail
          (Class|CharacterBase|ChangeState (Variables|Default|GetMyCharacter) "/Game/Project/Blueprints/Monster/FMonsterState.FMonsterState" "Chase"))))
    (:2
      (Utilities|DistancetoPlayer 3e+02
        (:Success
          (Animation|Montage|PlayMontage (Variables|Default|GetMyMesh) "/Game/Hyun_BossCharacter/Animations/Hetto_Attack01Strong_Montage.Hetto_Attack01Strong_Montage"
            (:OnBlendOut
              (Class|CharacterBase|ChangeState (Variables|Default|GetMyCharacter) "/Game/Project/Blueprints/Monster/FMonsterState.FMonsterState" "Dodge")
              (goto _label_2))))
        (:Fail
          (Class|CharacterBase|ChangeState (Variables|Default|GetMyCharacter) "/Game/Project/Blueprints/Monster/FMonsterState.FMonsterState" "Chase"))))))