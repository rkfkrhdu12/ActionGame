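; Monster AI state for a jump chase attack that leaps up, then lunges at the player.
; Montage notifies drive the launches: up into Flying, then a distance-scaled hop in Falling.
; After a short delay it raises gravity and launches horizontally toward a point offset along the player's velocity.
; A looping timer traces for ground, plays the landing montage, then switches to Observe on blend out.
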(event EventOnDelayFinished
  (bind _returnvalue (Class|UserdefinedState|GetActorLocation))
  (bind _returnvalue_2 (Class|UserdefinedMonsterState|GetPlayerLocation))
  (bind _myplayercharacter (Variables|Default|GetMyPlayerCharacter))
  (bind _charactermovement (Variables|/Script/Engine.Character|GetCharacterMovement _myplayercharacter))
  (bind _velocity (Variables|/Script/Engine.MovementComponent|GetVelocity _charactermovement))
  (bind _returnvalue_3 (Math|Vector|Normalize _velocity))
  (bind _returnvalue_4 (* _returnvalue_3 1e+02))
  (bind _returnvalue_5 (+ _returnvalue_2 (Math|Vector|MakeVector (.x _returnvalue_4) (.y _returnvalue_4) 0.0)))
  (bind _returnvalue_6 (- _returnvalue_5 _returnvalue))
  (bind _returnvalue_7 (Class|KismetMathLibrary|VectorNormal2D _returnvalue_6 0.0001))
  (bind _returnvalue_8 (* _returnvalue_7 1.4e+03))
  (Utilities|FlowControl|Sequence
    (:then_0
      (bind _returnvalue_9 (Class|UserdefinedState|IsValidTimer (Variables|Default|GetGroundCheckLoopHandle)))
      (if _returnvalue_9
        (bind _outhitresult (Class|CharacterBase|LineTrace (Variables|Default|GetMyCharacter) (Class|UserdefinedState|GetActorLocation) (+ (Class|UserdefinedState|GetActorLocation) "0.000000,0.000000,-200.000000") "ECC_WorldStatic"))
        (if (.bblockinghit _outhitresult)
          (Animation|Montage|PlayMontage (Variables|Default|GetMyMesh) "/Game/Hyun_BossCharacter/Animations/Hetto_JumpChaseAttack_End_Montage.Hetto_JumpChaseAttack_End_Montage"
            (:then
              (Class|UserdefinedState|ClearTimer (Variables|Default|GetGroundCheckLoopHandle)))
            (:OnBlendOut
              (Class|CharacterBase|ChangeState (Variables|Default|GetMyCharacter) "/Game/Project/Blueprints/Monster/FMonsterState.FMonsterState" "Observe"))))))
    (:then_1
      (bind _returnvalue_10 (Class|UserdefinedState|IsValidTimer (stale EventOnAnimNotify _timerhandle)))
      (if _returnvalue_10
        (Variables|/Script/Engine.CharacterMovementComponent|SetGravityScale (Variables|Default|GetCharacter%20Movement) 3.0)
        (Character|LaunchCharacter (Variables|Default|GetMyCharacter) (Math|Vector|MakeVector (.x _returnvalue_8) (.y _returnvalue_8) 0.0) true false)
        (bind _timerhandle (Class|UserdefinedState|StartDelay 0.1 true))
        (Variables|Default|SetGroundCheckLoopHandle _timerhandle)))))

(event EventOnEnable
  (bind _character_movement (Variables|Default|GetCharacter%20Movement))
  (Variables|Default|SetDefault%20Movement%20Mode (Variables|/Script/Engine.CharacterMovementComponent|GetMovementMode _character_movement))
  (Variables|Default|SetDefault%20Gravity%20Scale (Variables|/Script/Engine.CharacterMovementComponent|GetGravityScale _character_movement))
  (AI|Navigation|StopMovement (Variables|Default|GetMyAIController))
  (CallFunction|LookatPlayer)
  (Animation|Montage|PlayMontage (Variables|Default|GetMyMesh) "/Game/Hyun_BossCharacter/Animations/Hetto_JumpChaseAttack_Start_Montage.Hetto_JumpChaseAttack_Start_Montage"))

(event EventOnDisable
  (Variables|/Script/Engine.CharacterMovementComponent|SetMaxWalkSpeed (Variables|Default|GetCharacter%20Movement) (Variables|Default|GetDefaultWalkSpeed))
  (Pawn|Components|CharacterMovement|SetMovementMode (Variables|Default|GetCharacter%20Movement) (Variables|Default|GetDefault%20Movement%20Mode) 0))

(event EventOnAnimNotify
  (params (DataTableRef :type Data%20Table%20Object%20Reference) (SelectedRowName :type Name :default "None") (EventReference :type Anim%20Notify%20Event%20Reference%20Structure%20%28by%20ref%29))
  (Utilities|FlowControl|Sequence
    (:then_0
      (bind _returnvalue (Class|CharacterBase|IsCompareTableData (Variables|Default|GetMyCharacter) "/Game/Project/Blueprints/Monster/FMonsterNotify.FMonsterNotify" "Attack_Jump_Jumping" SelectedRowName))
      (if _returnvalue
        (Character|LaunchCharacter (Variables|Default|GetMyCharacter) "0.000000,0.000000,1000.000000" true true)
        (Pawn|Components|CharacterMovement|SetMovementMode (Variables|Default|GetCharacter%20Movement) "MOVE_Flying" 0)))
    (:then_1
      (bind _returnvalue_2 (Class|CharacterBase|IsCompareTableData (Variables|Default|GetMyCharacter) "/Game/Project/Blueprints/Monster/FMonsterNotify.FMonsterNotify" "Attack_Jump_Go" SelectedRowName))
      (if _returnvalue_2
        (Pawn|Components|CharacterMovement|SetMovementMode (Variables|Default|GetCharacter%20Movement) "MOVE_Falling" 0)
        (Character|LaunchCharacter (Variables|Default|GetMyCharacter) (Math|Vector|MakeVector 0.0 0.0 (Math|Float|Clamp(Float) (* (Class|UserdefinedMonsterState|GetDistancetoPlayer) 0.6) 3e+02 7e+02)) true true)
        (bind _timerhandle (Class|UserdefinedState|StartDelay 0.2))))))

(event EventBeginPlay
  (Variables|Default|SetCharacter%20Movement (Variables|/Script/Engine.Character|GetCharacterMovement (Variables|Default|GetMyCharacter))))