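; Monster AI state that sidesteps relative to the player for a short random delay, then switches to the AttackNormal state.
; Patrol repeatedly issues short moves perpendicular to the direction toward the player, restarting whenever a move finishes.
; Controller yaw is off while observing, then restored with a look at the player before attacking.
; Tick, marked for deprecation, periodically randomizes the left or right direction.
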(event Custom|Patrol
  (bind _mycharacter (Variables|Default|GetMyCharacter))
  (bind _returnvalue (Transformation|GetActorLocation _mycharacter))
  (Class|UserdefinedMonsterState|OnMovetoLocation (+ _returnvalue (* (Math|Vector|GetRightVector (Math|Rotator|FindLookatRotation _returnvalue (Class|UserdefinedMonsterState|GetPlayerLocation))) 1e+02 (Math|Float|SelectFloat -1.0 1.0 (Variables|상태체크|GetIsMoveRight))))))

(event EventOnEnable
  (AI|Navigation|StopMovement (Variables|Default|GetMyAIController))
  (Variables|/Script/Engine.Pawn|SetbUseControllerRotationYaw (Variables|Default|GetMyMonsterCharacter) false)
  (CallFunction|Patrol)
  (bind _timerhandle (Class|UserdefinedState|StartDelay (* (Math|Float|Min(Float) (Math|Random|RandomFloat) 0.3) 7.0))))

(event EventTick
  (params (DeltaTime :type Float%20%28single-precision%29))
  ;[0.15 0.15 0.15 0.5] 폐기 예정
  (Utilities|FlowControl|Sequence
    (:then_1
      (CallFunction|UpdateMoveDirection DeltaTime))))

(event EventOnMoveFinished
  (params (bIsSuccess :type Boolean))
  (CallFunction|Patrol))

(event EventOnDelayFinished
  (bind _returnvalue (Class|UserdefinedState|IsValidTimer (stale EventOnEnable _timerhandle)))
  (if _returnvalue
    (Variables|/Script/Engine.Pawn|SetbUseControllerRotationYaw (Variables|Default|GetMyMonsterCharacter) true)
    (CallFunction|LookatPlayer)
    (Class|CharacterBase|ChangeState (Variables|Default|GetMyCharacter) "/Game/Project/Blueprints/Monster/FMonsterState.FMonsterState" "AttackNormal")))

(fn UpdateMoveDirection
  (params (DeltaTime :type Float%20%28double-precision%29))
  (bind _output_get (Variables|상태체크|SetMoveDirectionUpdateTime (+ DeltaTime (Variables|상태체크|GetMoveDirectionUpdateTime))))
  (if (> _output_get (LocalVariables|GetInterval))
    (Variables|상태체크|SetMoveDirectionUpdateTime 0.0)
    (Variables|상태체크|SetIsMoveRight (Math|Random|RandomBool))))