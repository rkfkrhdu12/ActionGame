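; BP_PlayerState_Idle is the player's idle state, which responds to movement and look input.
; On BeginPlay, once the IsValidCheck macro passes its IsValidValues test, it binds events to the InputManager's move-direction and look-direction inputs.
; Those events forward their values to Move and Look.
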(event Custom|MoveEvent
  (params (Value :type Vector%202D%20Structure))
  (CallFunction|Move Value))

(event Custom|LookEvent
  (params (Value :type Vector%202D%20Structure))
  (CallFunction|Look Value))

(event EventBeginPlay
  (bind _inputmanager (Variables|Default|GetInputManager))
  (|IsValidCheck
    (:exit
      (EventDispatchers|BindEventtoOnInputMoveDirection _inputmanager (delegate Custom|MoveEvent))
      (EventDispatchers|BindEventtoOnInputLookDirection _inputmanager (delegate Custom|LookEvent)))))