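; BP_PlayerState_Dash is the player's dash state in a character state machine.
; It caches the latest move-input direction from the controller, then on enable snaps the character's yaw to face it and plays the dash montage.
; When the montage blends out it switches to Idle, and CanChanged only permits transitions to Idle, checked against the FPlayerState data table.
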(event Custom|OnInputMoveDirection_이벤트
  (params (Value :type Vector%202D%20Structure))
  (Variables|Default|SetMoveDirection Value))

(event EventOnEnable
  (bind _movedirection (Variables|Default|GetMoveDirection))
  (Transformation|SetActorRotation (Variables|Default|GetMyCharacter) (Math|Rotator|MakeRotator 0.0 0.0 (.yaw (Math|Conversions|RotationFromXVector (Math|Vector|MakeVector (.x _movedirection) (.y _movedirection) 0.0)))) true)
  (Animation|Montage|PlayMontage (Variables|Default|GetMyMesh) "/Game/Player/Animation/Player_Dash_Montage.Player_Dash_Montage"
    (:OnBlendOut
      (Class|UserdefinedPlayerStateBase|ChangeCharacterState "/Game/Project/Blueprints/Player/FPlayerState.FPlayerState" "Idle"))))

(event EventBeginPlay
  (EventDispatchers|AssignOnInputMoveDirection (Variables|Default|GetMyPlayerController) (delegate Custom|OnInputMoveDirection_이벤트)))

(fn CanChanged
  (params (NextState :type Name%20%28by%20ref%29 :default "None"))
  (bind _returnvalue (Class|CharacterBase|IsCompareTableData "/Game/Project/Blueprints/Player/FPlayerState.FPlayerState" "Idle" NextState))
  (return _returnvalue))