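; Player state Blueprint for the parry, the opening phase of a block.
; On enable it disables player movement, sets IsBlocking and plays the block start montage.
; Releasing the Parry input clears IsBlocking without interrupting the montage.
; The ParryEnd anim notify, matched against the FPlayerNotify table, switches to Block if the flag is still set, otherwise to Idle.
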(event EventOnEnable
  (Variables|/Script/ActionGame.PlayerControllerBase|SetIsCanMove (Variables|Default|GetMyPlayerController) false)
  (Variables|Default|SetIsBlocking true)
  (Animation|Montage|PlayMontage (Variables|Default|GetMyMesh) "/Game/Player/Animation/Player_BlockStart_Montage.Player_BlockStart_Montage"))

(event EventOnInputKey
  (params (Type :type EPlayerInputType%20Enum :default "Move") (bValue :type Boolean))
  (switch Utilities|FlowControl|Switch|SwitchonEPlayerInputType Type
    (:Parry
      (if (not bValue)
        (Variables|Default|SetIsBlocking false)))))

(event EventOnAnimNotify
  (params (DataTableRef :type Data%20Table%20Object%20Reference) (SelectedRowName :type Name :default "None") (EventReference :type Anim%20Notify%20Event%20Reference%20Structure%20%28by%20ref%29))
  (Utilities|FlowControl|Sequence
    (:then_0
      (bind _returnvalue (Class|CharacterBase|IsCompareTableData "/Game/Project/Blueprints/Player/FPlayerNotify.FPlayerNotify" "ParryEnd" SelectedRowName))
      (if _returnvalue
        (if (Variables|Default|GetIsBlocking)
          (Class|UserdefinedPlayerStateBase|ChangeCharacterState "/Game/Project/Blueprints/Player/FPlayerState.FPlayerState" "Block")
          (else
            (Class|UserdefinedPlayerStateBase|ChangeCharacterState "/Game/Project/Blueprints/Player/FPlayerState.FPlayerState" "Idle")))))))