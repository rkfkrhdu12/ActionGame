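; Player attack state, filed as old, that plays a two-stage melee montage combo on enable and returns to Idle.
; Each stage plays a start montage, then branches to a normal or strong follow-up, with the second stage gated by IsNextAttackEnable.
; AttackCheck notifies flag an input window, but the logic that reads attack input to choose branches is disconnected, leaving Tick and blend events empty.
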(event EventOnEnable
  (CallFunction|IsCheckValues)
  ;[0.15 0.15 0.15 0.5] 공격 사이클
  (bind _notifyname (Animation|Montage|PlayMontage (Variables|Default|GetMyMesh) "/Game/Player/Old/Old/Animations/Player_Attack01_Start_Montage.Player_Attack01_Start_Montage") ; AttackStart
    (:OnCompleted
      (if (Variables|Default|GetIsNormalAttack)
        (Animation|Montage|PlayMontage (Variables|Default|GetMyMesh) "/Game/Player/Old/Old/Animations/Player_Attack01_Normal_Montage.Player_Attack01_Normal_Montage" ; NormalAttack
          (:OnCompleted
            (if (Variables|Default|GetIsNextAttackEnable)
              (bind _notifyname_2 (Animation|Montage|PlayMontage (Variables|Default|GetMyMesh) "/Game/Player/Old/Old/Animations/Player_Attack02_Start_Montage.Player_Attack02_Start_Montage" :!label _label) ; AttackStart
                (:OnBlendOut
                  (if (Variables|Default|GetIsNormalAttack)
                    (Animation|Montage|PlayMontage (Variables|Default|GetMyMesh) "/Game/Player/Old/Old/Animations/Player_Attack02_Normal_Montage.Player_Attack02_Normal_Montage"
                      (:OnBlendOut
                        (Class|UserdefinedState|ChangeState "Idle" :!label _label_2)
                        (Development|PrintString 0 "Normal")))
                    (else
                      (Animation|Montage|PlayMontage (Variables|Default|GetMyMesh) "/Game/Player/Old/Old/Animations/Player_Attack02_Strong_Montage.Player_Attack02_Strong_Montage"
                        (:OnBlendOut
                          (Class|UserdefinedState|ChangeState "Idle" :!label _label_3)
                          (Development|PrintString 0 "Strong"))))))
                (:OnNotifyBegin
                  (if (== _notifyname_2 "AttackCheck")
                    (Variables|Default|SetIsAttackCheck true))))
              (else
                (goto _label_2)))))
        (else
          (Animation|Montage|PlayMontage (Variables|Default|GetMyMesh) "/Game/Player/Old/Old/Animations/Player_Attack01_Strong_Montage.Player_Attack01_Strong_Montage" ; StrongAttack
            (:OnCompleted
              (if (Variables|Default|GetIsNextAttackEnable)
                (goto _label)
                (else
                  (goto _label_3))))))))
    (:OnNotifyBegin
      (if (== _notifyname "AttackCheck")
        (Variables|Default|SetIsAttackCheck true)))))

(event EventTick
  (params (DeltaTime :type Float%20%28single-precision%29)))

(event EventOnAnimBlendOut
  (params (Montage :type Anim%20Montage%20Object%20Reference) (bInterrupted :type Boolean)))

(event EventOnAnimBlendin
  (params (Montage :type Anim%20Montage%20Object%20Reference)))