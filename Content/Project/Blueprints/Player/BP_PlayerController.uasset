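; Player controller that turns input events into movement, camera look and state changes on the player character.
; BeginPlay binds handlers for move, look, attack, parry, dash and target input, with move and look gated by permission flags.
; Attack, parry and dash request named states from a player state table, with parry refused during Block or Parry.
; Target input toggles a look-at mode that changes walk speed and camera speed.
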(event Custom|OnInputAttack_이벤트
  (params (InputValue :type Boolean))
  ;[1 1 1 0.5] 키 입력
  ;;[1 1 1 0.5] 공격 입력
  (if InputValue
    (Class|CharacterBase|ChangeState (Variables|Default|GetMyCharacter) "/Game/Project/Blueprints/Player/FPlayerState.FPlayerState" "Attack")))

(event Custom|OnInputParry_이벤트
  (params (InputValue :type Boolean))
  ;[1 1 1 0.5] 키 입력
  ;;[1 1 1 0.5] 패링 입력
  (bind _isnotblock_parry (|IsNotBlockParry)
    (:Next
      (if (and _isnotblock_parry InputValue)
        (Class|CharacterBase|ChangeState (Variables|Default|GetMyCharacter) "/Game/Project/Blueprints/Player/FPlayerState.FPlayerState" "Parry")))))

(event Custom|OnInputLookDirection_이벤트
  (params (Value :type Vector%202D%20Structure))
  ;[1 1 1 0.5] 키 입력
  ;;[1 1 1 0.5] 카메라 이동 입력
  (if (Variables|Default|GetbCanMoveCamera)
    (CallFunction|Look Value)))

(event Custom|OnInputDash_이벤트
  (params (InputValue :type Boolean))
  ;[1 1 1 0.5] 키 입력
  ;;[1 1 1 0.5] 대시 입력
  (if InputValue
    (Class|CharacterBase|ChangeState (Variables|Default|GetMyCharacter) "/Game/Project/Blueprints/Player/FPlayerState.FPlayerState" "Dash")))

(event Custom|OnInputLookAtTarget_이벤트
  (params (InputValue :type Boolean))
  ;[1 1 1 0.5] 키 입력
  ;;[0.781 1 0.9075 0.5] 타게팅 입력
  (if InputValue
    (Variables|Default|SetbIsLookAtTarget (not (Variables|Default|GetbIsLookAtTarget)))
    (CallFunction|Lookat)))

(event Custom|OnInputMoveDirection_이벤트
  (params (Value :type Vector%202D%20Structure))
  ;[1 1 1 0.5] 키 입력
  ;;[1 1 1 0.5] 이동 입력
  (if (Variables|Default|GetbCanMove)
    (Class|CharacterBase|Move (Variables|Default|GetMyCharacter) Value)))

(event EventBeginPlay
  (Utilities|FlowControl|Sequence
    (:then_0
      ;[1 1 1 0.5] 키 입력
      ;;[1 1 1 0.5] 이동 입력
      (EventDispatchers|AssignOnInputMoveDirection (delegate Custom|OnInputMoveDirection_이벤트))
      ;;[1 1 1 0.5] 카메라 이동 입력
      (EventDispatchers|AssignOnInputLookDirection (delegate Custom|OnInputLookDirection_이벤트))
      ;;[1 1 1 0.5] 공격 입력
      (EventDispatchers|AssignOnInputAttack (delegate Custom|OnInputAttack_이벤트))
      ;;[1 1 1 0.5] 패링 입력
      (EventDispatchers|AssignOnInputParry (delegate Custom|OnInputParry_이벤트))
      ;;[1 1 1 0.5] 대시 입력
      (EventDispatchers|AssignOnInputDash (delegate Custom|OnInputDash_이벤트))
      ;;[0.781 1 0.9075 0.5] 타게팅 입력
      (EventDispatchers|AssignOnInputLookatTarget (delegate Custom|OnInputLookAtTarget_이벤트)))))

(fn ConstructionScript)

(fn Look
  (params (InputValue :type Vector%202D%20Structure))
  (bind _mousemovespeed (Variables|Default|GetMouseMoveSpeed))
  (bind _currentcameraspeed (Variables|Default|GetCurrentCameraSpeed))
  (bind _returnvalue (* _mousemovespeed 0.8))
  (|CameraMove(Yaw) (* (.x InputValue) _returnvalue _currentcameraspeed))
  (|CameraMove(Pitch) (* (.y InputValue) _returnvalue _currentcameraspeed)))

(fn Lookat
  (Class|PlayerCharacterBase|OnLookatMode (Variables|Default|GetMyCharacter))
  (if (Variables|Default|GetbIsLookAtTarget)
    (Variables|/Script/Engine.CharacterMovementComponent|SetMaxWalkSpeed (Variables|/Script/Engine.Character|GetCharacterMovement (Variables|Default|GetMyCharacter)) (Variables|LookAt|GetLookAtMode_MoveSpeed))
    (Variables|Default|SetCurrentCameraSpeed (Variables|LookAt|GetLookatMode_CameraSpeed))
    (Utilities|IsValid (Variables|Default|GetLookAtTarget))
    (else
      (Variables|Default|SetCurrentCameraSpeed 1.0)
      (Variables|/Script/Engine.CharacterMovementComponent|SetMaxWalkSpeed (Variables|/Script/Engine.Character|GetCharacterMovement (Variables|Default|GetMyCharacter)) 6e+02))))